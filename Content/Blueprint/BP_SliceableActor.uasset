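; BP_SliceableActor is an actor that can be cut into physics-driven halves through RequestSlice.
; On BeginPlay it copies its static mesh into a procedural mesh and hides the original.
; RequestSlice checks state, count and a time window, then slices hit components listed in SlicePieces, capping cuts and pushing halves apart.
; New halves are not added to SlicePieces, and FinalizeProcessing, called by timer or slice limit, is empty.
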(event EventBeginPlay
  (bind _slicepieces (Variables|Default|GetslicePieces))
  (bind _proceduralmesh (Variables|Default|GetProceduralMesh))
  (bind _staticmesh (Variables|Default|GetStaticMesh))
  (Development|SetHiddeninGame (Variables|Default|GetProceduralMesh) true true)
  (if (Variables|Default|GetbCanBeSliced)
    (Class|KismetProceduralMeshLibrary|CopyProceduralMeshfromStaticMeshComponent (Variables|Default|GetStaticMesh) 0 _proceduralmesh true)
    (Rendering|Material|SetMaterial _proceduralmesh 0 (Rendering|Material|GetMaterial _staticmesh 0))
    (Development|SetHiddeninGame _staticmesh true true)
    (Collision|SetCollisionEnabled _staticmesh "NoCollision")
    (Development|SetHiddeninGame _proceduralmesh false false)
    (Collision|SetCollisionEnabled _proceduralmesh "QueryAndPhysics")
    (Variables|Default|SetbRuntimeMeshReady true)
    (Utilities|Array|Clear _slicepieces)
    (Utilities|Array|Add _slicepieces (Variables|Default|GetProceduralMesh))))

(event EventRequestSlice
  (params (slicePlanePosition :type Vector :default "0, 0, 0") (slicePlaneNormal :type Vector :default "0, 0, 0") (hitComp :type Primitive%20Component%20Object%20Reference) (sliceInstigator :type Actor%20Object%20Reference) (impulseStrenght :type Float%20%28double-precision%29))
  (bind _returnvalue (Utilities|Time|GetGameTimeinSeconds))
  (bind _returnvalue_2 (Math|Vector|Normalize slicePlaneNormal))
  (if (Variables|Default|GetbRuntimeMeshReady)
    (if (Variables|Default|GetbCanBeSliced)
      (if (not (Variables|Default|GetbIsFinalized))
        (if (< (Variables|Default|GetcurrentNumberSliced) (Variables|Default|GetmaxNumberSliced))
          (if (< (- _returnvalue (Variables|Default|GetlastTimeSliced)) (Variables|Default|GetsliceCooldown))
            (Variables|Default|SetlastTimeSliced _returnvalue)
            (Math|Integer|IncrementInt (Variables|Default|GetcurrentNumberSliced)
              (:%20%20
                (Utilities|IsValid hitComp
                  (:Is%20Valid
                    (bind _asprocedural_mesh_component (Utilities|Casting|CastToProceduralMeshComponent hitComp))
                    (if (Utilities|Array|ContainsItem (Variables|Default|GetslicePieces) _asprocedural_mesh_component)
                      (bind _output_get (Variables|Default|SettargetProcMesh _asprocedural_mesh_component))
                      (bind _outotherhalfprocmesh (Class|KismetProceduralMeshLibrary|SliceProceduralMesh _output_get slicePlanePosition _returnvalue_2 true "CreateNewSectionForCap" (Variables|Default|GetsliceCapMaterial)))
                      (Physics|SetSimulatePhysics (Variables|Default|GettargetProcMesh) true)
                      (Class|PrimitiveComponent|WakeAllRigidBodies (Variables|Default|GettargetProcMesh))
                      (Physics|AddImpulse (Variables|Default|GettargetProcMesh) (* _returnvalue_2 impulseStrenght) "None" false)
                      (Utilities|IsValid _outotherhalfprocmesh
                        (:Is%20Valid
                          (Physics|SetSimulatePhysics _outotherhalfprocmesh true)
                          (Class|PrimitiveComponent|WakeAllRigidBodies _outotherhalfprocmesh)
                          (Collision|SetCollisionEnabled _outotherhalfprocmesh "QueryAndPhysics")
                          (Physics|AddImpulse _outotherhalfprocmesh (* (* _returnvalue_2 -1) impulseStrenght) "None" false)
                          (Utilities|Time|ClearandInvalidateTimerbyHandle (Variables|Default|GetfinalizeTimerHandle))
                          (Utilities|Time|SetTimerbyFunctionName 0 "finalizeProcessing" (Variables|Default|GetfinalizeDelay))))
                      (else
                        (Variables|Default|SettargetProcMesh (Variables|Default|GetProceduralMesh)))))
                  (:Is%20Not%20Valid
                    (Variables|Default|SettargetProcMesh (Variables|Default|GetProceduralMesh))))))
            (else
              (Development|PrintString "CD slice time")))
          (else
            (CallFunction|FinalizeProcessing)))
        (else
          (Development|PrintString "item is finalized")))
      (else
        (Development|PrintString "Can't be sliced ")))
    (else
      (Development|PrintString "procedural mesh not ready"))))

(fn ConstructionScript)

(fn FinalizeProcessing)